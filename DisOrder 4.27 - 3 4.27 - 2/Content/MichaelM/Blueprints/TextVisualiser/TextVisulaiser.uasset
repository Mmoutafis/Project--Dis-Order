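; Trigger-volume actor that visualises player-entered text as a Niagara effect.
; Overlapping its box shows the W_TextVisualiser widget, whose commit event supplies the text, cell size and column count.
; It draws the text centred in red on a render target sized from column count and text length, then feeds that texture and grid parameters to Niagara and resets the system.
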(event `self.ReceiveBeginPlay`
  (bind _returnvalue (`|CreateWidget` "/Game/MichaelM/Blueprints/TextVisualiser/W_TextVisualiser.W_TextVisualiser_C" (`GameplayStatics.GetPlayerController` 0)))
  (bind _output_get (set `self.InputWidget` _returnvalue))
  (add `/Game/MichaelM/Blueprints/TextVisualiser/W_TextVisualiser.TextCommited` _output_get (`|CreateDelegate` :!event `TextCommited_Event_0`)))

(event `TextCommited_Event_0`
  (params (`Text Render` :type String) (CellSize :type "Float (double-precision)") (XCount :type Integer))
  (bind _xcount (`self.XCount`))
  (bind _niagara (`self.Niagara`))
  (bind _rendertarget (`self.RenderTarget`))
  (bind _returnvalue (`KismetStringLibrary.Len` (`self.TextRender`)))
  (bind _returnvalue_2 (/ (`KismetMathLibrary.Conv_IntToDouble` (`self.XCount`)) (* (`KismetMathLibrary.Conv_IntToDouble` (`KismetStringLibrary.Len` (`self.TextRender`))) 8.0)))
  (bind _returnvalue_3 (`KismetMathLibrary.Round` (* (/ (`KismetMathLibrary.Conv_IntToDouble` _xcount) (`KismetMathLibrary.Conv_IntToDouble` _returnvalue)) 2.0)))
  (`|ExecutionSequence`
    (:`then_0`
      (set `self.TextRender` `Text Render`))
    (:`then_1`
      (set `self.CellSize` CellSize))
    (:`then_2`
      (set `self.XCount` XCount))
    (:`then_3`
      (if (> _returnvalue 0)
        (`|ExecutionSequence`
          (:`then_0`
            (bind _returnvalue_4 (`KismetRenderingLibrary.CreateRenderTarget2D` _xcount _returnvalue_3))
            (set `self.RenderTarget` _returnvalue_4)
            (`NiagaraComponent.SetVariableFloat` _niagara "CellSize" (`self.CellSize`))
            (`NiagaraComponent.SetVariableInt` _niagara "XCount" (`self.XCount`))
            (`NiagaraComponent.SetVariableInt` _niagara "ZCount" _returnvalue_3)
            (`NiagaraFunctionLibrary.SetTextureObject` _niagara "Texture" (`self.RenderTarget`)))
          (:`then_1`
            (`KismetRenderingLibrary.ClearRenderTarget2D` _rendertarget)
            (bind (_canvas _size _context) (`KismetRenderingLibrary.BeginDrawCanvasToRenderTarget` _rendertarget))
            (`Canvas.K2_DrawText` _canvas "/Engine/EngineFonts/Roboto.Roboto" (`self.TextRender`) (* _size 0.5) (`KismetMathLibrary.MakeVector2D` _returnvalue_2 _returnvalue_2) (struct :`R` 1.0 :`A` 1.0) 0.0 (struct :`A` 1.0) (0.0 0.0) true true false (struct :`A` 1.0))
            (`KismetRenderingLibrary.EndDrawCanvasToRenderTarget` _context)
            (`NiagaraComponent.ResetSystem` (`self.Niagara`))))))))

(event `self.Box.OnComponentBeginOverlap`
  (params (OverlappedComponent :type "PrimitiveComponent Object Reference") (OtherActor :type "Actor Object Reference") (OtherComp :type "PrimitiveComponent Object Reference") (OtherBodyIndex :type Integer) (bFromSweep :type Boolean) (SweepResult :type "HitResult Structure (by ref)"))
  (`UserWidget.AddToViewport` (`self.InputWidget`) 0))

(event `self.Box.OnComponentEndOverlap`
  (params (OverlappedComponent :type "PrimitiveComponent Object Reference") (OtherActor :type "Actor Object Reference") (OtherComp :type "PrimitiveComponent Object Reference") (OtherBodyIndex :type Integer))
  (`Widget.RemoveFromParent` (`self.InputWidget`)))

(fn `UserConstructionScript`)