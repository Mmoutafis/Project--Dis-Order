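; BP_Enemy is an enemy NPC that damages the player on contact and dissolves when its health runs low.
; A box overlap with PlayerCharacterTest applies fixed damage, gated by a DoOnce that resets after a short delay as a hit cooldown.
; Incoming damage reduces Health; below a threshold the enemy slows, disables collision and plays a timeline driving a dynamic material's Appearance parameter before destroying itself.
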(event `self.ReceiveActorBeginOverlap`
  (params (OtherActor :type "Actor Object Reference")))

(event `self.Box.OnComponentBeginOverlap`
  (params (OverlappedComponent :type "PrimitiveComponent Object Reference") (OtherActor :type "Actor Object Reference") (OtherComp :type "PrimitiveComponent Object Reference") (OtherBodyIndex :type Integer) (bFromSweep :type Boolean) (SweepResult :type "HitResult Structure (by ref)"))
  (bind _asplayer_character_test (cast `/Game/MichaelM/Blueprints/PlayerCharacterTest` OtherActor))
  (`/Engine/EditorBlueprintResources/StandardMacros.DoOnce` false :!label _label
    (:`Completed`
      (`GameplayStatics.ApplyDamage` _asplayer_character_test 10.0)
      (`KismetSystemLibrary.Delay` 1.0)
      (`KismetSystemLibrary.PrintString` "Hit")
      (goto _label :!via `Reset`))))

(event `self.ReceiveAnyDamage`
  (params (Damage :type "Float (single-precision)") (DamageType :type "DamageType Object Reference") (InstigatedBy :type "Controller Object Reference") (DamageCauser :type "Actor Object Reference"))
  (set `self.Health` (- (`self.Health`) Damage))
  (if (< (`self.Health`) 10.0)
    (set `CharacterMovementComponent.MaxWalkSpeed` 50.0 (`self.CharacterMovement`))
    (`self.SetActorEnableCollision` false)
    (bind _returnvalue (`PrimitiveComponent.CreateDynamicMaterialInstance` (`self.Mesh`) 0 "/Game/MichaelM/Materials/M_Negative_Thoughts_Main_Inst.M_Negative_Thoughts_Main_Inst" "None"))
    (bind (_direction _newtrack_0) (`Timeline|Dissolve`)
      (:`Update`
        (`MaterialInstanceDynamic.SetScalarParameterValue` _returnvalue "Appearance" _newtrack_0))
      (:`Finished`
        (`self.K2_DestroyActor`)))))

(fn `UserConstructionScript`)