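; BP_PositiveThought_M is a pickup with a spinning sphere that the player collects by overlapping its box collider.
; Overlap disables collision and animates the sphere's dynamic material "Appearance" parameter through a timeline.
; It then increments and prints the game mode's PositiveThoughtCount, which selects one of two timelines driving Player_collection's "Emissive Mult".
; That timeline's update also destroys the actor, so it ends on its first update.
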(event `self.ReceiveTick`
  (params (DeltaSeconds :type "Float (single-precision)"))
  (bind _sphere (`self.Sphere`))
  (bind (_relativerotation_roll _relativerotation_pitch _relativerotation_yaw) (`KismetMathLibrary.BreakRotator` (`SceneComponent.RelativeRotation` _sphere)))
  (`SceneComponent.K2_SetRelativeRotation` _sphere (`KismetMathLibrary.MakeRotator` (+ _relativerotation_roll 2.0) _relativerotation_pitch _relativerotation_yaw) false false))

(event `self.BoxCollider.OnComponentBeginOverlap`
  (params (OverlappedComponent :type "PrimitiveComponent Object Reference") (OtherActor :type "Actor Object Reference") (OtherComp :type "PrimitiveComponent Object Reference") (OtherBodyIndex :type Integer) (bFromSweep :type Boolean) (SweepResult :type "HitResult Structure (by ref)"))
  (cast `/Game/MichaelM/Blueprints/PlayerCharacterTest` OtherActor)
  (`self.SetActorEnableCollision` false)
  (bind _returnvalue (`PrimitiveComponent.CreateDynamicMaterialInstance` (`self.Sphere`) 0 "/Game/MichaelM/Materials/M_Positive_Thoughts_Main_Inst.M_Positive_Thoughts_Main_Inst" "None"))
  (bind (_direction _newtrack_0) (`Timeline|Timeline_0`)
    (:`Update`
      (`MaterialInstanceDynamic.SetScalarParameterValue` _returnvalue "Appearance" _newtrack_0))
    (:`Finished`
      (bind _astop_down_game_mode_1 (cast `/Game/MichaelM/Blueprints/TopDownGameMode1` (`GameplayStatics.GetGameMode`)))
      (bind _output_get (set `self.Positive Thought Count` (`/Game/MichaelM/Blueprints/TopDownGameMode1.Positive Thought Count` _astop_down_game_mode_1)))
      (bind _output_get_2 (set `/Game/MichaelM/Blueprints/TopDownGameMode1.Positive Thought Count` (+ _output_get 1.0) _astop_down_game_mode_1))
      (`KismetSystemLibrary.PrintString` (`KismetStringLibrary.Conv_DoubleToString` _output_get_2))
      (bind _returnvalue_2 (`KismetMaterialLibrary.GetScalarParameterValue` "/Game/MichaelM/Materials/Player_collection.Player_collection" "Emissive Mult"))
      (set `self.Emmisive Mult` _returnvalue_2)
      (if (>= (`self.Positive Thought Count`) 1.0)
        (bind (_direction_2 _newtrack_0_2) (`Timeline|Timeline_2`)
          (:`Update`
            (`KismetMaterialLibrary.SetScalarParameterValue` "/Game/MichaelM/Materials/Player_collection.Player_collection" "Emissive Mult" _newtrack_0_2)
            (`self.K2_DestroyActor`)))
        (else
          (bind (_direction_3 _newtrack_0_3) (`Timeline|Timeline_1`)
            (:`Update`
              (`KismetMaterialLibrary.SetScalarParameterValue` "/Game/MichaelM/Materials/Player_collection.Player_collection" "Emissive Mult" _newtrack_0_3)
              (`self.K2_DestroyActor`))))))))

(fn `UserConstructionScript`)