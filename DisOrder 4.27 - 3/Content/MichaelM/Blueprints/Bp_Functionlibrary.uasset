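; Blueprint function library providing a search for the nearest actor of a given class to a target location.
; It gathers every actor of that class and loops through them, comparing each one's distance to the location against a running minimum held in local variables.
; It returns the closest recorded actor and its distance.
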(fn `Find Nearest Actor of Class`
  (params (Class :type "Actor Class Reference") (`Target Location` :type "Vector Structure"))
  (returns (`Nearest Actor` :type "Actor Object Reference") (`Nearest Distance` :type "Float (double-precision)"))
  (locals (Loc_Nearest_Actor :type "Actor Object Reference") (Loc_Nearest_Distance :type "Float (double-precision)" :default 10000.0))
  (bind _outactors (`GameplayStatics.GetAllActorsOfClass` null Class))
  (for _array_element _outactors
    (bind _returnvalue (`KismetMathLibrary.Vector_Distance` (`Actor.K2_GetActorLocation` _array_element) (`local.Target Location`)))
    (if (< _returnvalue (`local.Loc_Nearest_Distance`))
      (set `local.Loc_Nearest_Distance` _returnvalue)
      (set `local.Loc_Nearest_Actor` _array_element)))
  (return (`local.Loc_Nearest_Actor`) (`local.Loc_Nearest_Distance`)))