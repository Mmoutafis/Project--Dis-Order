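; Top-down player character with cursor-facing movement, montage-driven sword attack and dodge, wall climbing and health.
; Each tick fans line traces into a vision cone, draws it as triangles to a render target, and publishes player position to a material parameter collection.
; Health steps shorten the cone, and low health slows walking.
; Tick traces also detect walls, switching to Flying for climbing, with interact-triggered ledge climb-up and Space to let go.
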(event `Key|LeftMouseButton`
  (params (Key :type "Key Structure"))
  ;[1 1 1] Attack
  (:`Pressed`
    (if (`self.Attacking?`)
      _
      (elif (not (`self.Is Movement Locked?`))
        (set `self.bCanBeDamaged` false)
        (set `self.Is dodge locked?` true)
        (set `self.Attacking?` true)
        (`|PlayMontage` (`self.Mesh`) "/Game/MichaelM/Animations/Stable_Sword_Inward_Slash__1__mixamo_com1_Montage.Stable_Sword_Inward_Slash__1__mixamo_com1_Montage" 1.5
          (:`OnCompleted`
            _)
          (:`OnBlendOut`
            _)
          (:`OnInterrupted`
            _))
        (set `self.Attacking?` false)
        (set `self.Is dodge locked?` false)
        (set `self.bCanBeDamaged` true)
        (`GameplayStatics.ApplyDamage` null 10.0)))))

(event `self.ReceiveBeginPlay`
  ;[1 1 1] Set Walk Speed & Weapon Owner
  (`self.SetOwner` (`ChildActorComponent.ChildActor` (`self.ChildActor`)) self)
  (set `CharacterMovementComponent.MaxWalkSpeed` 250.0 (`self.CharacterMovement`)))

(event `self.ReceiveAnyDamage`
  (params (Damage :type "Float (single-precision)") (DamageType :type "DamageType Object Reference") (InstigatedBy :type "Controller Object Reference") (DamageCauser :type "Actor Object Reference"))
  (bind _charactermovement (`self.CharacterMovement`))
  ;[1 1 1] Taking Damage
  (bind _output_get (set `self.Health` (- (`self.Health`) Damage)))
  (if (<= _output_get 0.0)
    (`/Engine/EditorBlueprintResources/StandardMacros.DoOnce` false
      (:`Completed`
        (`self.PlayAnimMontage` "/Game/MichaelM/Animations/Standing_React_Small_From_Front_mixamo_com1_Montage.Standing_React_Small_From_Front_mixamo_com1_Montage")
        (`KismetSystemLibrary.PrintString` "Fully effected")
        (`self.DisableInput` null)
        (`KismetSystemLibrary.Delay` 0.3)
        (`self.EnableInput` null)))
    (else
      (`self.PlayAnimMontage` "/Game/MichaelM/Animations/Standing_React_Small_From_Front_mixamo_com1_Montage.Standing_React_Small_From_Front_mixamo_com1_Montage")
      (`KismetSystemLibrary.PrintString` "Player Hit")
      (`self.DisableInput` null)
      (`KismetSystemLibrary.Delay` 0.3)
      (`self.EnableInput` null)
      (if (<= (`self.Health`) 50.0)
        (set `self.Injured?` true)
        (set `CharacterMovementComponent.MaxWalkSpeed` 100.0 _charactermovement)
        (else
          (set `self.Injured?` false)
          (set `CharacterMovementComponent.MaxWalkSpeed` 250.0 _charactermovement))))))

(event `self.ReceiveTick`
  (params (DeltaSeconds :type "Float (single-precision)"))
  (`self.LOSVisionsystem`)
  (`self.Light Length System`)
  (if (not (`self.Is Climbing Up`))
    (`self.Climb System`)))

(event `InputAction|Dodge`
  (params (Key :type "Key Structure"))
  (bind (_returnvalue_x _returnvalue_y) (`KismetMathLibrary.BreakVector` (* (`self.GetActorForwardVector`) (`self.Move Distance`))))
  (bind (_velocity_x _velocity_y _velocity_z) (`KismetMathLibrary.BreakVector` (`MovementComponent.Velocity` (`self.CharacterMovement`))))
  ;[1 1 1] Dodge
  (:`Pressed`
    (if (not (`self.Is Movement Locked?`))
      (if (not (`self.Attacking?`))
        (if (`self.Is dodge locked?`)
          _
          (elif (not (`self.Is Climbing?`))
            (set `self.Is Movement Locked?` true)
            (`|PlayMontage` (`self.Mesh`) "/Game/MichaelM/Animations/DodgeBackward_Inplace_Montage.DodgeBackward_Inplace_Montage"
              (:`then`
                (bind (_direction _distance_multiplier) (`Timeline|Movement` :!via `PlayFromStart`)
                  (:`Update`
                    (set `MovementComponent.Velocity` (`KismetMathLibrary.MakeVector` _returnvalue_x _returnvalue_y _velocity_z) (`self.CharacterMovement`)))))
              (:`OnCompleted`
                (set `self.Is Movement Locked?` false :!label _label))
              (:`OnInterrupted`
                (goto _label)))))))))

(event `InputAction|Interact`
  (params (Key :type "Key Structure"))
  ;[1 1 1] Movement & climb
  (:`Pressed`
    (if (`self.Is Climbing?`)
      (if (not (`self.Is on ledge?`))
        (set `self.Is Climbing Up` true)
        (set `self.Is Climbing?` false)
        (set `self.Is Movement Locked?` true)
        (bind _returnvalue (`self.PlayAnimMontage` "/Game/ClimbRetargetedAnims/Climbing_ClimbUpAtTop_RM_Montage.Climbing_ClimbUpAtTop_RM_Montage"))
        (`KismetSystemLibrary.Delay` _returnvalue)
        (set `self.Is Climbing Up` false)
        (`CharacterMovementComponent.SetMovementMode` (`self.CharacterMovement`) "MOVE_Walking" 0 :!label _label_2)
        (set `self.Is Movement Locked?` false)))))

(event `InputAxis|MoveForward`
  (params (AxisValue :type "Float (single-precision)"))
  ;[1 1 1] Movement & climb
  (set `self.MoveForward/Down` AxisValue)
  (if (not (`self.Is Movement Locked?`))
    (if (`self.Is Climbing?`)
      (if true
        (`self.AddMovementInput` (`self.GetActorUpVector` (`GameplayStatics.GetPlayerCharacter` 0)) AxisValue)
        (else
          (set `self.MoveForward/Down` 0.0)))
      (else
        (`self.AddMovementInput` (90.0 0.0 0.0) AxisValue)
        (`self.Rotate To Face Cursor` :!label _label_3)))))

(event `InputAxis|MoveRight`
  (params (AxisValue :type "Float (single-precision)"))
  ;[1 1 1] Movement & climb
  (set `self.MoveRight/Left` AxisValue)
  (if (not (`self.Is Movement Locked?`))
    (if (`self.Is Climbing?`)
      (`self.AddMovementInput` (`KismetMathLibrary.GetRightVector` (`self.K2_GetActorRotation`)) AxisValue)
      (else
        (`self.AddMovementInput` (0.0 90.0 0.0) AxisValue)
        (goto _label_3)))))

(event `Key|SpaceBar`
  (params (Key :type "Key Structure"))
  (bind (_returnvalue_x _returnvalue_y) (`KismetMathLibrary.BreakVector` (* (`KismetMathLibrary.GetForwardVector` (struct)) -300.0)))
  ;[1 1 1] Movement & climb
  (:`Pressed`
    (if (`self.Is Climbing?`)
      (`self.LaunchCharacter` (`KismetMathLibrary.MakeVector` _returnvalue_x _returnvalue_y))
      (goto _label_2))))

(event `InputAction|Interact`
  (params (Key :type "Key Structure"))
  ;[1 1 1] Movement & climb
  (:`Pressed`
    (if (`self.Can Climb?`)
      (if (`self.Climbing`)
        (set `self.Climbing` false)
        (`CharacterMovementComponent.SetMovementMode` (`self.CharacterMovement`) "MOVE_Walking" 0)
        (else
          (set `self.Climbing` true))))))

(fn `Climb System`
  (bind _returnvalue (`self.K2_GetActorLocation`))
  (bind _capsulecomponent (`self.CapsuleComponent`))
  (bind _returnvalue_2 (`SceneComponent.K2_GetComponentLocation` _capsulecomponent))
  (bind _outactors (`GameplayStatics.GetAllActorsWithTag` (`self.No Climb Tag`)))
  (bind (_outhit _returnvalue_3) (`KismetSystemLibrary.LineTraceSingle` _returnvalue_2 (+ (+ _returnvalue_2 (0.0 0.0 100.0)) (* (`SceneComponent.GetForwardVector` _capsulecomponent) 45.0)) "TraceTypeQuery1" true _outactors))
  (if _returnvalue_3
    (bind (_outhit_2 _returnvalue_4) (`KismetSystemLibrary.LineTraceSingle` :`Start` _returnvalue :`End` (+ (+ _returnvalue (0.0 0.0 110.0)) (* (`SceneComponent.GetForwardVector` (`self.CapsuleComponent`)) 45.0)) :`TraceChannel` "TraceTypeQuery1" :`bTraceComplex` true :`TraceColor` (struct :`G` 0.145682 :`B` 1.0 :`A` 1.0)))
    (set `self.Is on ledge?` _returnvalue_4)
    (bind (_returnvalue_roll _returnvalue_pitch _returnvalue_yaw) (`KismetMathLibrary.BreakRotator` (`KismetMathLibrary.Conv_VectorToRotator` (`.Normal` (`GameplayStatics.BreakHitResult` _outhit)))))
    (`self.K2_SetActorRotation` (`KismetMathLibrary.MakeRotator` 0.0 0.0 (+ _returnvalue_yaw 180.0)))
    (`/Engine/EditorBlueprintResources/StandardMacros.DoOnce` false :!label _label
      (:`Completed`
        (set `self.Is Climbing?` true)
        (`CharacterMovementComponent.SetMovementMode` (`self.CharacterMovement`) "MOVE_Flying" 0)
        (set `CharacterMovementComponent.bOrientRotationToMovement` false (`self.CharacterMovement`))))
    (elif (`self.Is Climbing?`)
      (set `self.Is Climbing?` false)
      (`CharacterMovementComponent.SetMovementMode` (`self.CharacterMovement`) "MOVE_Walking" 0)
      (goto _label :!via `Reset`))))

(fn `Create Cone`
  (bind _returnvalue (`self.K2_GetActorLocation`))
  (bind _traceresults (`self.TraceResults`))
  (`KismetArrayLibrary.Array_Clear` (`self.TraceResults`))
  (for _index (range (+ (`self.NumTraces`) 1))
    (bind _returnvalue_2 (`KismetMathLibrary.GreaterGreater_VectorRotator` (`KismetMathLibrary.GreaterGreater_VectorRotator` (`self.GetActorForwardVector`) (`KismetMathLibrary.MakeRotator` 0.0 0.0 (/ (* (`self.NumTraces`) (`self.DegresPerTrace`)) -2.0))) (`KismetMathLibrary.MakeRotator` 0.0 0.0 (* _index (`self.DegresPerTrace`)))))
    (bind _returnvalue_3 (+ (* _returnvalue_2 (`self.Light Length`)) _returnvalue))
    (bind (_outhit _returnvalue_4) (`KismetSystemLibrary.LineTraceSingle` _returnvalue _returnvalue_3 "TraceTypeQuery1"))
    (if _returnvalue_4
      (bind _returnvalue_5 (* _returnvalue_2 10.0))
      (`KismetArrayLibrary.Array_Add` _traceresults (+ _returnvalue_5 (`.Location` (`GameplayStatics.BreakHitResult` _outhit))))
      (else
        (`KismetArrayLibrary.Array_Add` _traceresults (+ _returnvalue_5 _returnvalue_3))))))

(fn `Light Length System`
  (if (== (`self.Health`) 100.0)
    (set `self.Light Length` 600.0)
    (elif (== (`self.Health`) 90.0)
      (set `self.Light Length` 550.0)
      (elif (== (`self.Health`) 80.0)
        (set `self.Light Length` 500.0)
        (elif (== (`self.Health`) 70.0)
          (set `self.Light Length` 450.0)
          (elif (== (`self.Health`) 60.0)
            (set `self.Light Length` 400.0)
            (elif (== (`self.Health`) 50.0)
              (set `self.Light Length` 350.0)
              (elif (== (`self.Health`) 40.0)
                (set `self.Light Length` 300.0)
                (elif (== (`self.Health`) 30.0)
                  (set `self.Light Length` 250.0)
                  (elif (== (`self.Health`) 20.0)
                    (set `self.Light Length` 200.0)
                    (elif (== (`self.Health`) 10.0)
                      (set `self.Light Length` 150.0))))))))))))

(fn `LOSVisionsystem`
  (bind _los_render_target (`self.LOS Render Target`))
  (`|ExecutionSequence`
    (:`then_0`
      (`KismetMaterialLibrary.SetVectorParameterValue` "/Game/MichaelM/Materials/FogOfWarMat/PlayerPosition.PlayerPosition" "PlayerPosition" (`KismetMathLibrary.Conv_VectorToLinearColor` (`self.K2_GetActorLocation`))))
    (:`then_1`
      (`self.Create Cone`))
    (:`then_2`
      (`self.PrepareTrianglesForCanvas`))
    (:`then_3`
      (`KismetRenderingLibrary.ClearRenderTarget2D` _los_render_target)
      (bind (_canvas _size _context) (`KismetRenderingLibrary.BeginDrawCanvasToRenderTarget` _los_render_target))
      (`Canvas.K2_DrawTriangle` _canvas null (`self.CanvasTriangles`))
      (`KismetRenderingLibrary.EndDrawCanvasToRenderTarget` _context))))

(fn `PrepareTrianglesForCanvas`
  (bind _returnvalue (`self.K2_GetActorLocation`))
  (bind _returnvalue_2 (`KismetMathLibrary.MakeVector` 900.0 900.0))
  (bind _traceresults (`self.TraceResults`))
  (`KismetArrayLibrary.Array_Clear` (`self.CanvasTriangles`))
  (for _index (range (+ (- (`KismetArrayLibrary.Array_Length` (`self.TraceResults`)) 2) 1))
    (`KismetArrayLibrary.Array_Add` (`self.CanvasTriangles`) (make `CanvasUVTri` (`KismetMathLibrary.Conv_VectorToVector2D` _returnvalue_2) (0.0 0.0) (struct :`R` 1.0 :`G` 1.0 :`B` 1.0) (`KismetMathLibrary.Conv_VectorToVector2D` (+ (- (`|GetArrayItem` _traceresults _index) _returnvalue) _returnvalue_2)) (0.0 0.0) (struct :`R` 1.0 :`G` 1.0 :`B` 1.0) (`KismetMathLibrary.Conv_VectorToVector2D` (+ (- (`|GetArrayItem` _traceresults (+ _index 1)) _returnvalue) _returnvalue_2)) (0.0 0.0) (struct :`R` 1.0 :`G` 1.0 :`B` 1.0)))))

(fn `Rotate To Face Cursor`
  (bind _returnvalue (`GameplayStatics.GetPlayerController` 0))
  (bind (_returnvalue_roll _returnvalue_pitch _returnvalue_yaw) (`KismetMathLibrary.BreakRotator` (`KismetMathLibrary.FindLookAtRotation` (`self.K2_GetActorLocation`) (`.Location` (`GameplayStatics.BreakHitResult` (`PlayerController.GetHitResultUnderCursorByChannel` _returnvalue "TraceTypeQuery1" true))))))
  (`Controller.SetControlRotation` _returnvalue (`KismetMathLibrary.MakeRotator` 0.0 0.0 _returnvalue_yaw)))

(fn `UserConstructionScript`)