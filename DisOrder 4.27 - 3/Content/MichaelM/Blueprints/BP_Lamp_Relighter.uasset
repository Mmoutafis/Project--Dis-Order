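; BP_Lamp_Relighter is a lamp interaction point meant to heal the player when relit.
; A box overlap with PlayerCharacterTest shows the EToRelight prompt and sets NearCandle, and leaving reverses both.
; Pressing F while near sets the lamp's own Health copy, read from the player at BeginPlay, to full and prints "healed", without writing back to the player.
; LOSSystem is an empty stub.
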(event `self.ReceiveBeginPlay`
  (bind _asplayer_character_test (cast `/Game/MichaelM/Blueprints/PlayerCharacterTest` (`GameplayStatics.GetPlayerCharacter` 0)))
  (set `self.Health` (`/Game/MichaelM/Blueprints/PlayerCharacterTest.Health` _asplayer_character_test)))

(event `self.ReceiveTick`
  (params (DeltaSeconds :type "Float (single-precision)")))

(event `Key|F`
  (params (Key :type "Key Structure"))
  (:`Pressed`
    (if (`self.Near Candle?`)
      (set `self.Health` 100.0)
      (`KismetSystemLibrary.PrintString` "healed"))))

(event `self.Box.OnComponentBeginOverlap`
  (params (OverlappedComponent :type "PrimitiveComponent Object Reference") (OtherActor :type "Actor Object Reference") (OtherComp :type "PrimitiveComponent Object Reference") (OtherBodyIndex :type Integer) (bFromSweep :type Boolean) (SweepResult :type "HitResult Structure (by ref)"))
  (cast `/Game/MichaelM/Blueprints/PlayerCharacterTest` OtherActor)
  (`SceneComponent.SetHiddenInGame` (`self.E to relight`) false false)
  (set `self.Near Candle?` true))

(event `self.Box.OnComponentEndOverlap`
  (params (OverlappedComponent :type "PrimitiveComponent Object Reference") (OtherActor :type "Actor Object Reference") (OtherComp :type "PrimitiveComponent Object Reference") (OtherBodyIndex :type Integer))
  (cast `/Game/MichaelM/Blueprints/PlayerCharacterTest` OtherActor)
  (`SceneComponent.SetHiddenInGame` (`self.E to relight`) true false)
  (set `self.Near Candle?` false))

(fn `LOSSystem`)

(fn `UserConstructionScript`)