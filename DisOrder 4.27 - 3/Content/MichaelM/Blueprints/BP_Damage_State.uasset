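; BP_Damage_State is an animation notify state that marks the window in an animation during which the player's weapon is active.
; On begin and end, it casts the mesh owner to PlayerCharacterTest and gets the BP_Weapon from its ChildActor component.
; It calls WeaponActive at the start and WeaponDeactivated at the end, doing nothing if either cast fails.
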(fn `Received_NotifyBegin`
  (params (MeshComp :type "SkeletalMeshComponent Object Reference") (Animation :type "AnimSequenceBase Object Reference") (TotalDuration :type "Float (double-precision)"))
  (returns (ReturnValue :type Boolean))
  (bind _asplayer_character_test (cast `/Game/MichaelM/Blueprints/PlayerCharacterTest` (`ActorComponent.GetOwner` MeshComp)))
  (bind _asbp_weapon (cast `/Game/MichaelM/Blueprints/BP_Weapon` (`ChildActorComponent.ChildActor` (`/Game/MichaelM/Blueprints/PlayerCharacterTest.ChildActor` _asplayer_character_test))))
  (`/Game/MichaelM/Blueprints/BP_Weapon.Weapon Active` _asbp_weapon)
  (return false))

(fn `Received_NotifyEnd`
  (params (MeshComp :type "SkeletalMeshComponent Object Reference") (Animation :type "AnimSequenceBase Object Reference"))
  (returns (ReturnValue :type Boolean))
  (bind _asplayer_character_test (cast `/Game/MichaelM/Blueprints/PlayerCharacterTest` (`ActorComponent.GetOwner` MeshComp)))
  (bind _asbp_weapon (cast `/Game/MichaelM/Blueprints/BP_Weapon` (`ChildActorComponent.ChildActor` (`/Game/MichaelM/Blueprints/PlayerCharacterTest.ChildActor` _asplayer_character_test))))
  (`/Game/MichaelM/Blueprints/BP_Weapon.Weapon Deactivated` _asbp_weapon)
  (return false))