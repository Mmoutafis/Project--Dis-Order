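; BP_PathTracer_Colored draws a path as consecutive colored segments, from runtime-supplied points or an editor-edited outline spline in ManualEditMode.
; DrawColoredPath cuts the points by each ColoredDistances length, with the last segment taking the remainder unless LimitDraw is set.
; Segments are pooled BP_PathTracer child actors, colored from ColoredPathColors, with end fades and indents only at the outer ends.
; A separate tracer instance spans the first and last drawn points for start/end marks.
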(event `self.ReceiveBeginPlay`
  (set `self.ManualEditMode` false))

(fn `DrawColoredPath`
  (params (PathPoints :type "Array of Vector Structure (by ref)") (ColoredDistances :type "Array of Float (double-precision) (by ref)"))
  (locals (IndexLOCAL :type Integer) (LastPointLOCAL :type "Vector Structure") (PathPointsLOCAL :type "Array of Vector Structure"))
  (bind _pathpointslocal (`local.PathPointsLOCAL`))
  (if (and (> (`KismetArrayLibrary.Array_Length` (`self.ColoredPathColors`)) 0) (> (`KismetArrayLibrary.Array_Length` PathPoints) 1) (> (`KismetArrayLibrary.Array_Length` ColoredDistances) 0))
    (set `self.ColoredSegmetsLength` ColoredDistances)
    (for (_array_element _array_index) (`self.ColoredSegmetsLength`)
      (if (< _array_element 0.01)
        (`KismetArrayLibrary.Array_Remove` (`self.ColoredSegmetsLength`) _array_index)))
    (if (> (`KismetArrayLibrary.Array_Length` (`self.ColoredSegmetsLength`)) 0)
      (set `self.PathPoints` PathPoints)
      (set `local.PathPointsLOCAL` PathPoints)
      (set `self.PathsUsingAmount` 0)
      (for _array_element_2 (`self.Paths`)
        (`self.SetActorHiddenInGame` _array_element_2 true))
      (set `self.ColoredSegmentsAmount` (`KismetArrayLibrary.Array_Length` (`self.ColoredSegmetsLength`)))
      (for _index (range (`self.ColoredSegmentsAmount`))
        (set `local.IndexLOCAL` _index)
        (if (or (!= (`local.IndexLOCAL`) (- (`self.ColoredSegmentsAmount`) 1)) (`self.LimitDraw`))
          (bind (_partofpath _pathremainder _hasremainder) (`self.FindPathByLength` (`|GetArrayItem` (`self.ColoredSegmetsLength`) (`local.IndexLOCAL`)) (`local.PathPointsLOCAL`)))
          (set `self.LastSegment` (not _hasremainder))
          (bind _path (`self.GetPath` (`local.IndexLOCAL`)))
          (`/Game/PathTracer/Blueprints/BP_PathTracer.DrawPath` _path _partofpath)
          (set `local.LastPointLOCAL` (`|GetArrayItem` _partofpath (`KismetArrayLibrary.Array_LastIndex` _partofpath)))
          (if (not (`self.LastSegment`))
            (set `local.PathPointsLOCAL` _pathremainder)
            (else
              (break)))
          (else
            (bind _path_2 (`self.GetPath` (`local.IndexLOCAL`)))
            (`/Game/PathTracer/Blueprints/BP_PathTracer.DrawPath` _path_2 _pathpointslocal)
            (set `local.LastPointLOCAL` (`|GetArrayItem` _pathpointslocal (`KismetArrayLibrary.Array_LastIndex` _pathpointslocal))))))
      (`/Game/PathTracer/Blueprints/BP_PathTracer.DrawPath` (`self.PathTracer`) (`|MakeArray` (`|GetArrayItem` (`self.PathPoints`)) (`local.LastPointLOCAL`))))))

(fn `FindPathByLength`
  (params (Lenght :type "Float (double-precision)") (PathPoints :type "Array of Vector Structure (by ref)"))
  (returns (PartOfPath :type "Array of Vector Structure") (PathRemainder :type "Array of Vector Structure") (HasRemainder :type Boolean))
  (locals (MaxDrawPathLengthLOCAL :type "Float (double-precision)") (WayPiontsPartialLOCAL :type "Array of Vector Structure") (MoveTargetLocationLOCAL :type "Vector Structure") (PathPointsLOCAL :type "Array of Vector Structure"))
  (bind _pathpointslocal (`local.PathPointsLOCAL`))
  (bind _returnvalue (`KismetArrayLibrary.Array_LastIndex` (`local.WayPiontsPartialLOCAL`)))
  (set `local.MaxDrawPathLengthLOCAL` Lenght)
  (set `local.PathPointsLOCAL` PathPoints)
  (`KismetArrayLibrary.Array_Add` (`local.WayPiontsPartialLOCAL`) (`|GetArrayItem` _pathpointslocal))
  (for _index (range (`KismetArrayLibrary.Array_LastIndex` _pathpointslocal))
    (bind _output (`|GetArrayItem` _pathpointslocal (+ _index 1)))
    (bind _output_2 (`|GetArrayItem` _pathpointslocal _index))
    (bind _returnvalue_2 (- _output _output_2))
    (bind _returnvalue_3 (- (`local.MaxDrawPathLengthLOCAL`) (`KismetMathLibrary.VSize` _returnvalue_2)))
    (if (>= _returnvalue_3 0.0)
      (`KismetArrayLibrary.Array_Add` (`local.WayPiontsPartialLOCAL`) _output)
      (set `local.MaxDrawPathLengthLOCAL` _returnvalue_3)
      (set `local.MoveTargetLocationLOCAL` _output)
      (else
        (bind _output_get (set `local.MoveTargetLocationLOCAL` (+ _output_2 (* (`KismetMathLibrary.Normal` _returnvalue_2) (`local.MaxDrawPathLengthLOCAL`)))))
        (`KismetArrayLibrary.Array_Add` (`local.WayPiontsPartialLOCAL`) _output_get)
        (for _ (range _returnvalue)
          (`KismetArrayLibrary.Array_Remove` (`local.PathPointsLOCAL`)))
        (`KismetArrayLibrary.Array_Insert` (`local.PathPointsLOCAL`) (`|GetArrayItem` (`local.WayPiontsPartialLOCAL`) _returnvalue))
        (return (`local.WayPiontsPartialLOCAL`) (`local.PathPointsLOCAL`) true))))
  (return (`local.PathPointsLOCAL`) _ false))

(fn `GetPath`
  (params (SegmentIndex :type Integer))
  (returns (Path :type "/Game/PathTracer/Blueprints/BP_PathTracer Object Reference"))
  (locals (SwgmentIndexLOCAL :type Integer) (PathLOCAL :type "/Game/PathTracer/Blueprints/BP_PathTracer Object Reference"))
  (bind _coloredpathcolors (`self.ColoredPathColors`))
  (bind _pathsusingamount (`self.PathsUsingAmount`))
  (bind _pathtracer (`self.PathTracer`))
  (bind _pathtracer_2 (`self.PathTracer`))
  (bind _returnvalue (`KismetArrayLibrary.Array_LastIndex` _coloredpathcolors))
  (bind _returnvalue_2 (- _pathsusingamount 1))
  (bind _output (`|GetArrayItem` (`self.Paths`) (- (`self.PathsUsingAmount`) 1)))
  (set `local.SwgmentIndexLOCAL` SegmentIndex)
  (`|ExecutionSequence`
    (:`then_0`
      (if (> (`KismetArrayLibrary.Array_Length` (`self.Paths`)) (`self.PathsUsingAmount`))
        (`/Engine/EditorBlueprintResources/StandardMacros.IncrementInt` (`self.PathsUsingAmount`)
          (:`  `
            (`self.SetActorHiddenInGame` _output false)
            (set `local.PathLOCAL` _output)))
        (else
          (bind _returnvalue_3 (`AddComponent|NODE_AddChildActorComponent-0` :`RelativeTransform` (`KismetMathLibrary.MakeTransform` (0.0 0.0 100.0))))
          (`ChildActorComponent.SetChildActorClass` _returnvalue_3 (`self.PathTracerClass`))
          (bind _asbp_path_tracer (cast `/Game/PathTracer/Blueprints/BP_PathTracer` (`ChildActorComponent.ChildActor` _returnvalue_3)))
          (`KismetArrayLibrary.Array_Add` (`self.Paths`) _asbp_path_tracer)
          (`/Engine/EditorBlueprintResources/StandardMacros.IncrementInt` (`self.PathsUsingAmount`)
            (:`  `
              (set `local.PathLOCAL` _asbp_path_tracer)
              (set `/Game/PathTracer/Blueprints/BP_PathTracer.PathColor` (`|GetArrayItem` _coloredpathcolors (`KismetMathLibrary.SelectInt` _returnvalue_2 (mod (- _pathsusingamount 2) _returnvalue) (>= _returnvalue _returnvalue_2))) (`local.PathLOCAL`))
              (set `/Game/PathTracer/Blueprints/BP_PathTracer.PathMarkStartClass` null (`local.PathLOCAL`))
              (set `/Game/PathTracer/Blueprints/BP_PathTracer.PathMarkEndClass` null (`local.PathLOCAL`)))))))
    (:`then_1`
      (if (== (`local.SwgmentIndexLOCAL`) 0)
        (set `/Game/PathTracer/Blueprints/BP_PathTracer.TranslucentStartSize` (`/Game/PathTracer/Blueprints/BP_PathTracer.TranslucentStartSize` _pathtracer_2) (`local.PathLOCAL`))
        (set `/Game/PathTracer/Blueprints/BP_PathTracer.StartPathIndent` (`/Game/PathTracer/Blueprints/BP_PathTracer.StartPathIndent` _pathtracer_2) (`local.PathLOCAL`))
        (else
          (set `/Game/PathTracer/Blueprints/BP_PathTracer.TranslucentStartSize` 0.0 (`local.PathLOCAL`))
          (set `/Game/PathTracer/Blueprints/BP_PathTracer.StartPathIndent` 0.0 (`local.PathLOCAL`)))))
    (:`then_2`
      (if (`self.LastSegment`)
        (set `/Game/PathTracer/Blueprints/BP_PathTracer.TranslucentEndSize` (`/Game/PathTracer/Blueprints/BP_PathTracer.TranslucentEndSize` _pathtracer) (`local.PathLOCAL`))
        (set `/Game/PathTracer/Blueprints/BP_PathTracer.EndPathIndent` (`/Game/PathTracer/Blueprints/BP_PathTracer.EndPathIndent` _pathtracer) (`local.PathLOCAL`))
        (return (`local.PathLOCAL`))
        (else
          (set `/Game/PathTracer/Blueprints/BP_PathTracer.TranslucentEndSize` 0.0 (`local.PathLOCAL`))
          (set `/Game/PathTracer/Blueprints/BP_PathTracer.EndPathIndent` 0.0 (`local.PathLOCAL`))
          (return (`local.PathLOCAL`)))))))

(fn `GetPathLength`
  (returns (PathLength :type "Float (double-precision)"))
  (locals (PathLengthLOCAL :type "Float (double-precision)" :default 0.0))
  (for _index (range (`self.PathsUsingAmount`))
    (set `local.PathLengthLOCAL` (+ (`/Game/PathTracer/Blueprints/BP_PathTracer.GetPathLength` (`|GetArrayItem` (`self.Paths`) _index)) (`local.PathLengthLOCAL`))))
  (return (`local.PathLengthLOCAL`)))

(fn `SetupOutlineSpline`
  (bind _outlinespline (`self.OutlineSpline`))
  (`KismetArrayLibrary.Array_Clear` (`self.PathPoints`))
  (for _index (range (`SplineComponent.GetNumberOfSplinePoints` (`self.OutlineSpline`)))
    (`SplineComponent.SetSplinePointType` _outlinespline _index "Linear" true)
    (`KismetArrayLibrary.Array_Add` (`self.PathPoints`) (`SplineComponent.GetLocationAtSplinePoint` _outlinespline _index "World"))))

(fn `SetupStartAndEndMarks`
  (bind _returnvalue (`AddComponent|NODE_AddChildActorComponent-5` :`RelativeTransform` (`KismetMathLibrary.MakeTransform` (0.0 0.0 100.0))))
  (`ChildActorComponent.SetChildActorClass` _returnvalue (`self.PathTracerClass`))
  (bind _asbp_path_tracer (cast `/Game/PathTracer/Blueprints/BP_PathTracer` (`ChildActorComponent.ChildActor` _returnvalue)))
  (bind _output_get (set `self.PathTracer` _asbp_path_tracer))
  (set `/Game/PathTracer/Blueprints/BP_PathTracer.PathType` "NewEnumerator7" _output_get)
  (`/Game/PathTracer/Blueprints/BP_PathTracer.DrawPath` (`self.PathTracer`) (`|MakeArray` (0.0 0.0 0.0) (100.0 0.0 0.0) :!type "Vector Structure")))

(fn `UpdatePathInRuntime`
  (bind _pathtracer (`self.PathTracer`))
  (for _array_element (`self.Paths`)
    (set `/Game/PathTracer/Blueprints/BP_PathTracer.PathMarkStartClass` null _array_element)
    (set `/Game/PathTracer/Blueprints/BP_PathTracer.PathMarkEndClass` null _array_element)
    (set `/Game/PathTracer/Blueprints/BP_PathTracer.LimitPath` false _array_element)
    (`/Game/PathTracer/Blueprints/BP_PathTracer.UpdatePathInRuntime` _array_element))
  (set `/Game/PathTracer/Blueprints/BP_PathTracer.PathType` "NewEnumerator7" _pathtracer)
  (set `/Game/PathTracer/Blueprints/BP_PathTracer.LimitPath` false _pathtracer)
  (`/Game/PathTracer/Blueprints/BP_PathTracer.UpdatePathInRuntime` _pathtracer))

(fn `UserConstructionScript`
  (if (`self.ManualEditMode`)
    (`self.SetupStartAndEndMarks`)
    (`self.SetupOutlineSpline`)
    (`self.DrawColoredPath` (`self.PathPoints`) (`self.ColoredDistances`))
    (else
      (`self.SetupStartAndEndMarks`))))