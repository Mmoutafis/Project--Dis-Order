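; Child fire point light Blueprint that scales its light intensity to the player character's health, dimming at lower values.
; BeginPlay runs the parent logic, casts the player to PlayerCharacterTest and copies Health once, with no later refresh in this file.
; Tick calls LightSystem, a nested exact-match check on health in steps of ten that sets PointLight intensity, leaving it unchanged for other values.
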(event `self.ReceiveBeginPlay`
  (`parent.ReceiveBeginPlay`)
  (bind _asplayer_character_test (cast `/Game/MichaelM/Blueprints/PlayerCharacterTest` (`GameplayStatics.GetPlayerCharacter` 0)))
  (set `self.As Player Character Test` _asplayer_character_test)
  (set `self.Health` (`/Game/MichaelM/Blueprints/PlayerCharacterTest.Health` (`self.As Player Character Test`))))

(event `self.ReceiveActorBeginOverlap`
  (params (OtherActor :type "Actor Object Reference")))

(event `self.ReceiveTick`
  (params (DeltaSeconds :type "Float (single-precision)"))
  (`self.Light_system`))

(fn `Light_system`
  (if (== (`self.Health`) 100.0)
    (`LightComponent.SetIntensity` (`self.PointLight`) 140.0)
    (elif (== (`self.Health`) 90.0)
      (`LightComponent.SetIntensity` (`self.PointLight`) 130.0)
      (elif (== (`self.Health`) 80.0)
        (`LightComponent.SetIntensity` (`self.PointLight`) 120.0)
        (elif (== (`self.Health`) 70.0)
          (`LightComponent.SetIntensity` (`self.PointLight`) 110.0)
          (elif (== (`self.Health`) 60.0)
            (`LightComponent.SetIntensity` (`self.PointLight`) 100.0)
            (elif (== (`self.Health`) 50.0)
              (`LightComponent.SetIntensity` (`self.PointLight`) 90.0)
              (elif (== (`self.Health`) 40.0)
                (`LightComponent.SetIntensity` (`self.PointLight`) 80.0)
                (elif (== (`self.Health`) 30.0)
                  (`LightComponent.SetIntensity` (`self.PointLight`) 20.0)
                  (elif (== (`self.Health`) 20.0)
                    (`LightComponent.SetIntensity` (`self.PointLight`) 10.0)
                    (elif (== (`self.Health`) 10.0)
                      (`LightComponent.SetIntensity` (`self.PointLight`) 10.0))))))))))))

(fn `UserConstructionScript`
  (`parent.UserConstructionScript`))