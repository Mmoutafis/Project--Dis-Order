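; BP_TestDummy is a test combat character that automatically plays a sword slash montage every three seconds.
; It retains player controls for axis movement, cursor-facing rotation and click-to-slash, and sets itself as owner of its child actor.
; Damage lowers Health, plays a hit reaction with a brief input lockout, and halves walk speed when injured.
; At zero Health the reaction fires only once, with no death logic.
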(event `InputAxis|MoveForward`
  (params (AxisValue :type "Float (single-precision)"))
  (`self.AddMovementInput` (90.0 0.0 0.0) AxisValue)
  (`self.Rotate To Face Cursor` :!label _label))

(event `InputAxis|MoveRight`
  (params (AxisValue :type "Float (single-precision)"))
  (`self.AddMovementInput` (0.0 90.0 0.0) AxisValue)
  (goto _label))

(event `Key|LeftMouseButton`
  (params (Key :type "Key Structure"))
  (:`Pressed`
    (`self.PlayAnimMontage` "/Game/MichaelM/Animations/Stable_Sword_Inward_Slash__1__mixamo_com1_Montage.Stable_Sword_Inward_Slash__1__mixamo_com1_Montage")))

(event `self.ReceiveAnyDamage`
  (params (Damage :type "Float (single-precision)") (DamageType :type "DamageType Object Reference") (InstigatedBy :type "Controller Object Reference") (DamageCauser :type "Actor Object Reference"))
  (bind _charactermovement (`self.CharacterMovement`))
  (bind _output_get (set `self.Health` (- (`self.Health`) Damage)))
  (if (<= _output_get 0.0)
    (`/Engine/EditorBlueprintResources/StandardMacros.DoOnce` false
      (:`Completed`
        (`self.PlayAnimMontage` "/Game/MichaelM/Animations/Standing_React_Small_From_Front_mixamo_com1_Montage.Standing_React_Small_From_Front_mixamo_com1_Montage")
        (`KismetSystemLibrary.PrintString` "Fully effected")
        (`self.DisableInput` null)
        (`KismetSystemLibrary.Delay` 0.3)
        (`self.EnableInput` null)))
    (else
      (`self.PlayAnimMontage` "/Game/MichaelM/Animations/Standing_React_Small_From_Front_mixamo_com1_Montage.Standing_React_Small_From_Front_mixamo_com1_Montage")
      (`KismetSystemLibrary.PrintString` "Player Hit")
      (`self.DisableInput` null)
      (`KismetSystemLibrary.Delay` 0.3)
      (`self.EnableInput` null)
      (if (<= (`self.Health`) 50.0)
        (set `self.Injured?` true)
        (set `CharacterMovementComponent.MaxWalkSpeed` 250.0 _charactermovement)
        (else
          (set `self.Injured?` false)
          (set `CharacterMovementComponent.MaxWalkSpeed` 500.0 _charactermovement))))))

(event `self.ReceiveBeginPlay`
  (`self.SetOwner` (`ChildActorComponent.ChildActor` (`self.ChildActor`)) self))

(event `self.ReceiveTick`
  (params (DeltaSeconds :type "Float (single-precision)"))
  (`/Engine/EditorBlueprintResources/StandardMacros.DoOnce` false :!label _label_2
    (:`Completed`
      (`self.PlayAnimMontage` "/Game/MichaelM/Animations/Stable_Sword_Inward_Slash__1__mixamo_com1_Montage.Stable_Sword_Inward_Slash__1__mixamo_com1_Montage")
      (`KismetSystemLibrary.Delay` 3.0)
      (goto _label_2 :!via `Reset`))))

(fn `Rotate To Face Cursor`
  (bind _returnvalue (`GameplayStatics.GetPlayerController` 0))
  (bind (_returnvalue_roll _returnvalue_pitch _returnvalue_yaw) (`KismetMathLibrary.BreakRotator` (`KismetMathLibrary.FindLookAtRotation` (`self.K2_GetActorLocation`) (`.Location` (`GameplayStatics.BreakHitResult` (`PlayerController.GetHitResultUnderCursorByChannel` _returnvalue "TraceTypeQuery1" true))))))
  (`Controller.SetControlRotation` _returnvalue (`KismetMathLibrary.MakeRotator` 0.0 0.0 _returnvalue_yaw)))

(fn `UserConstructionScript`)