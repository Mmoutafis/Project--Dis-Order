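; BP_Interactable is a trigger volume that lets the player character climb while inside it.
; CollisionBox begin overlap casts to PlayerCharacterTest and sets its CanClimb and ClimbUp flags.
; End overlap clears those two flags along with ClimbDown.
; An unconnected branch that would choose between climbing up and down never runs, so entering always enables upward climbing.
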(event `self.ReceiveBeginPlay`)

(event `self.Collision box.OnComponentBeginOverlap`
  (params (OverlappedComponent :type "PrimitiveComponent Object Reference") (OtherActor :type "Actor Object Reference") (OtherComp :type "PrimitiveComponent Object Reference") (OtherBodyIndex :type Integer) (bFromSweep :type Boolean) (SweepResult :type "HitResult Structure (by ref)"))
  (bind _asplayer_character_test (cast `/Game/MichaelM/Blueprints/PlayerCharacterTest` OtherActor))
  (bind _output_get (set `self.As Player Character Test` _asplayer_character_test))
  (set `/Game/MichaelM/Blueprints/PlayerCharacterTest.Can Climb?` true _output_get)
  (set `/Game/MichaelM/Blueprints/PlayerCharacterTest.Climb Up?` true _output_get))

(event `self.Collision box.OnComponentEndOverlap`
  (params (OverlappedComponent :type "PrimitiveComponent Object Reference") (OtherActor :type "Actor Object Reference") (OtherComp :type "PrimitiveComponent Object Reference") (OtherBodyIndex :type Integer))
  (bind _asplayer_character_test (cast `/Game/MichaelM/Blueprints/PlayerCharacterTest` OtherActor))
  (bind _output_get (set `self.As Player Character Test` _asplayer_character_test))
  (set `/Game/MichaelM/Blueprints/PlayerCharacterTest.Can Climb?` false _output_get)
  (set `/Game/MichaelM/Blueprints/PlayerCharacterTest.Climb Up?` false _output_get)
  (set `/Game/MichaelM/Blueprints/PlayerCharacterTest.Climb Down?` false _output_get))

(fn `UserConstructionScript`)